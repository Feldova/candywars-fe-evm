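; Blueprint function library for blockchain wallets, storing each wallet's private key in a save game slot named after the wallet.
; WalletExist checks the slot, WalletCreate generates a secp256k1 key and saves it in a B_WalletSaveGame, and WalletRead loads it back.
; The key is stored without encryption in the graph.
; The address helpers are unfinished: SaveWalletAddress re-saves the loaded slot without using Value, and ReadWalletAddress is empty.
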(fn WalletExist
  (params (WalletName :type String))
  (bind _returnvalue (SaveGame|DoesSaveGameExist WalletName))
  (return _returnvalue))

(fn WalletCreate
  (params (WalletName :type String))
  (bind _returnvalue (SaveGame|CreateSaveGameObject "/Game/MainMenu/blockchain/blueprints/B_WalletSaveGame.B_WalletSaveGame_C"))
  (bind (_privatekey _returnvalue_2) (Class|TSBCEncryptionFunctionLibrary|Secp256k1GeneratePrivateKey))
  (if _returnvalue_2
    (Variables|/Game/MainMenu/blockchain/blueprints/B_WalletSaveGame.B_WalletSaveGame_C|SetWalletKey _returnvalue _privatekey)
    (bind _returnvalue_3 (SaveGame|SaveGametoSlot _returnvalue WalletName))
    (return _returnvalue_3)
    (else
      (return false))))

(fn WalletRead
  (params (WalletName :type String))
  (bind _returnvalue (SaveGame|LoadGamefromSlot WalletName))
  (bind _asb_wallet_save_game (Utilities|Casting|CastToB_WalletSaveGame _returnvalue)
    (:then
      (return true (Variables|/Game/MainMenu/blockchain/blueprints/B_WalletSaveGame.B_WalletSaveGame_C|GetWalletKey _asb_wallet_save_game)))
    (:CastFailed
      (return false 0))))

(fn SaveWalletAddress
  (params (KeyName :type String) (Value :type String))
  (bind _returnvalue (SaveGame|LoadGamefromSlot KeyName))
  (SaveGame|SaveGametoSlot _returnvalue KeyName))

(fn ReadWalletAddress
  (params (KeyName :type String)))