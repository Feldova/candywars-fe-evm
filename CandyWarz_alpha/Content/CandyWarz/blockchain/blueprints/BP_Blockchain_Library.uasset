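; Blueprint function library for CandyWarz that stores and reads blockchain wallet data in local save slots.
; Each wallet is a B_WalletSaveGame in a slot named after it, with functions to check existence, create it, save or read its address, and read its key.
; WalletCreate saves an empty address; its secp256k1 private key generation is disconnected, so no function here writes a generated key.
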(fn WalletExist
  (params (WalletName :type String))
  (bind _returnvalue (SaveGame|DoesSaveGameExist WalletName))
  (return _returnvalue))

(fn WalletCreate
  (params (WalletName :type String))
  (bind _returnvalue (SaveGame|CreateSaveGameObject "/Game/CandyWarz/blockchain/blueprints/B_WalletSaveGame.B_WalletSaveGame_C"))
  (Variables|/Game/CandyWarz/blockchain/blueprints/B_WalletSaveGame.B_WalletSaveGame_C|SetWalletAddress _returnvalue "")
  (bind _returnvalue_2 (SaveGame|SaveGametoSlot _returnvalue WalletName))
  (return _returnvalue_2))

(fn ByteWalletRead
  (params (WalletName :type String))
  (bind _returnvalue (SaveGame|LoadGamefromSlot WalletName))
  (bind _asb_wallet_save_game (Utilities|Casting|CastToB_WalletSaveGame _returnvalue)
    (:then
      (return true (Variables|/Game/CandyWarz/blockchain/blueprints/B_WalletSaveGame.B_WalletSaveGame_C|GetWalletKey _asb_wallet_save_game)))
    (:CastFailed
      (return false 0))))

(fn SaveWalletAddress
  (params (KeyName :type String) (Value :type String))
  (bind _returnvalue (SaveGame|LoadGamefromSlot KeyName))
  (bind _asb_wallet_save_game (Utilities|Casting|CastToB_WalletSaveGame _returnvalue))
  (Variables|/Game/CandyWarz/blockchain/blueprints/B_WalletSaveGame.B_WalletSaveGame_C|SetWalletAddress _asb_wallet_save_game Value)
  (SaveGame|SaveGametoSlot _returnvalue KeyName))

(fn ReadWalletAddress
  (params (KeyName :type String))
  (bind _returnvalue (SaveGame|LoadGamefromSlot KeyName))
  (bind _asb_wallet_save_game (Utilities|Casting|CastToB_WalletSaveGame _returnvalue)
    (:then
      (return (Variables|/Game/CandyWarz/blockchain/blueprints/B_WalletSaveGame.B_WalletSaveGame_C|GetWalletAddress _asb_wallet_save_game) true))
    (:CastFailed
      (return "" false))))